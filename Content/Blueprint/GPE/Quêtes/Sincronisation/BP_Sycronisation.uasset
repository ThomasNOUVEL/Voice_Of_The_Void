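; BP_Sycronisation is a quest prop with three LED components that show the progress of a synchronisation.
; Its Sycronisation event takes an Avancement value, selects Led3, Led2 or Led1 in that order, and swaps that LED's material to Mat_On.
; Each call changes a single LED, and nothing here switches one back off or calls the event.
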(event Custom|Sycronisation
  (params (Avancement :type Integer))
  (Rendering|Material|SetMaterial (Utilities|Select :Index Avancement :Option%200 (Variables|Default|GetLed%203) :Option%201 (Variables|Default|GetLed%202) :Option%202 (Variables|Default|GetLed%201) :Option%203 0) 0 "/Game/Blueprint/GPE/Quêtes/Sincronisation/Mat_On.Mat_On"))

(event EventBeginPlay
  (|CallParentFunction) ; This node is disabled and will not be called.\nDrag off pins to build functionality.
)

(event Collision|EventActorBeginOverlap
  (params (OtherActor :type Actor%20Object%20Reference))
  (|CallParentFunction OtherActor) ; This node is disabled and will not be called.\nDrag off pins to build functionality.
)

(event EventTick
  (params (DeltaSeconds :type Float%20%28single-precision%29))
  (|CallParentFunction DeltaSeconds) ; This node is disabled and will not be called.\nDrag off pins to build functionality.
)

(fn ConstructionScript
  (|CallParentFunction))