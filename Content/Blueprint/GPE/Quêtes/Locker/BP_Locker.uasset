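; BP_Locker is a quest gameplay element that controls the lock state of another object and displays it on a sphere.
; Its events store the target reference and set the lock state, swapping the sphere between on and off materials and forwarding the flag to the target through LockUnlockMessage.
; Breaking it sets a Break flag and shows the off material without messaging the target.
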(event Custom|Set%20loker%20information
  (params (Lock%20Unlock :type Boolean))
  (Rendering|Material|SetMaterial (Variables|Default|GetSphere) 0 (select Lock%20Unlock "/Game/Blueprint/GPE/Quêtes/Sincronisation/Mat_Off.Mat_Off" "/Game/Blueprint/GPE/Quêtes/Sincronisation/Mat_On.Mat_On"))
  (Class|BPILoker|LockUnlock(Message) (Variables|Default|GetObject%20Lock%20ref) Lock%20Unlock))

(event Custom|Set%20Object%20lock%20ref
  (params (Object%20Lock%20ref :type Actor%20Object%20Reference))
  (Variables|Default|SetObject%20Lock%20ref Object%20Lock%20ref))

(event EventBeginPlay
  (|CallParentFunction) ; This node is disabled and will not be called.\nDrag off pins to build functionality.
)

(event Collision|EventActorBeginOverlap
  (params (OtherActor :type Actor%20Object%20Reference))
  (|CallParentFunction OtherActor) ; This node is disabled and will not be called.\nDrag off pins to build functionality.
)

(event EventTick
  (params (DeltaSeconds :type Float%20%28single-precision%29))
  (|CallParentFunction DeltaSeconds) ; This node is disabled and will not be called.\nDrag off pins to build functionality.
)

(event EventBreaktheObject
  (Variables|Default|SetBreak true)
  (Rendering|Material|SetMaterial (Variables|Default|GetSphere) 0 "/Game/Blueprint/GPE/Quêtes/Sincronisation/Mat_Off.Mat_Off"))

(fn ConstructionScript
  (|CallParentFunction))