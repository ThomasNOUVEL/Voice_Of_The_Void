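; BP_QuestObject is an interactable world object that opens a quest UI once it has been broken.
; Breakobject sets the Break flag and changes the Cube's material.
; While broken, the first Interract creates the quest widget, stored as WBPClimatisationQuest, and passes it to the BP_GestionHUD actor found on BeginPlay.
; Later interactions ask that HUD manager to reopen the same widget.
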(event Custom|Break%20object
  (Variables|Default|SetBreak true)
  (Rendering|Material|SetMaterial (Variables|Default|GetCube) 0 0))

(event EventBeginPlay
  (|CallParentFunction)
  (bind _returnvalue (Actor|GetActorOfClass "/Game/Blueprint/Widgets/BP_GestionHUD.BP_GestionHUD_C"))
  (Variables|Default|SetGestion%20HUD%20ref _returnvalue))

(event Collision|EventActorBeginOverlap
  (params (OtherActor :type Actor%20Object%20Reference))
  (|CallParentFunction OtherActor) ; This node is disabled and will not be called.\nDrag off pins to build functionality.
)

(event EventTick
  (params (DeltaSeconds :type Float%20%28single-precision%29))
  (|CallParentFunction DeltaSeconds) ; This node is disabled and will not be called.\nDrag off pins to build functionality.
)

(event EventInterract
  (params (First%20person%20ref :type BP%20First%20Person%20Character%20Object%20Reference))
  (Variables|Default|SetFirst%20Person%20Ref First%20person%20ref)
  (if (Variables|Default|GetBreak)
    (if (Variables|Default|Getquest%20started)
      (Default|ReOppentheQuest (Variables|Default|GetGestion%20HUD%20ref) self (Variables|Default|GetWBP%20Climatisation%20Quest))
      (else
        (bind _returnvalue (UserInterface|CreateWidget (Variables|Default|GetClass)))
        (bind _output_get (Variables|Default|SetWBP%20Climatisation%20Quest _returnvalue))
        (Default|Quest (Variables|Default|GetGestion%20HUD%20ref) _output_get self)
        (Variables|Default|Setquest%20started true)))))

(fn ConstructionScript
  (|CallParentFunction))