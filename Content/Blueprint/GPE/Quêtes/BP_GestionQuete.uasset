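; Quest manager that periodically breaks random objects for the player to repair and punishes unfinished repairs by sending them to the backroom.
; A looping timer breaks a batch from the intact pool when none are outstanding, otherwise calls GoToBackroom on the player.
; Repair reports return objects to the pool and print remaining quests or completion.
; Lockers receive the break message once at startup, outside quest tracking.
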(event Custom|Break%20object
  (params (Target :type Actor%20Object%20Reference))
  (Development|PrintText (Utilities|Text|ToText(Object) Target) true true "(R=0.000000,G=0.660000,B=1.000000,A=1.000000)" 1e+01)
  (Class|BPIGestionReparation|BreaktheObject(Message) Target self)
  (Utilities|Array|RemoveItem (Variables|Default|GetAll%20quest%20Not%20breakArray) Target)
  (Utilities|Array|Add (Variables|Default|GetAll%20quest%20not%20finish) Target))

(event Custom|Select%20object%20to%20beak
  (bind _all_quest_not_breakarray (Variables|Default|GetAll%20quest%20Not%20breakArray))
  (if (Utilities|Array|IsEmpty (Variables|Default|GetAll%20quest%20not%20finish))
    (for _index (range 0 3)
      (if (not (Utilities|Array|IsEmpty _all_quest_not_breakarray))
        (CallFunction|BreakObject (.OutItem (Utilities|Array|Random _all_quest_not_breakarray)))))
    (else
      (Default|GotoBackroom (.AsBP%20First%20Person%20Character (Utilities|Casting|CastToBP_FirstPersonCharacter (Game|Player|GetPlayerPawn 0)))))))

(event Custom|Quest%20repared
  (params (ItemToFind :type Actor%20Object%20Reference%20%28by%20ref%29))
  (bind _all_quest_not_finish (Variables|Default|GetAll%20quest%20not%20finish))
  (if (Utilities|Array|ContainsItem _all_quest_not_finish ItemToFind)
    (Utilities|Array|RemoveItem _all_quest_not_finish ItemToFind)
    (Utilities|Array|Add (Variables|Default|GetAll%20quest%20Not%20breakArray) ItemToFind)
    (Development|PrintText (Utilities|Text|ToText(Object) ItemToFind) true true "(R=0.174314,G=1.000000,B=0.089963,A=1.000000)" 3.0)
    (Utilities|FlowControl|Delay 5.0)
    (if (Utilities|Array|IsEmpty (Variables|Default|GetAll%20quest%20not%20finish))
      (Development|PrintText "Finish !" true true "(R=0.049642,G=1.000000,B=0.000000,A=1.000000)" 3.0)
      (else
        (for _array_element (Variables|Default|GetAll%20quest%20not%20finish)
          (Development|PrintText (Utilities|Text|ToText(Object) _array_element) true true "(R=0.000000,G=0.660000,B=1.000000,A=1.000000)" 3.0))))))

(event EventBeginPlay
  (Variables|Default|SetAll%20quest%20Not%20breakArray (Variables|Default|GetAll%20quest%20Array))
  (Utilities|FlowControl|Delay 0.2)
  (CallFunction|SelectObjecttoBeak)
  (Utilities|Time|SetTimerbyEvent (delegate Custom|Select%20object%20to%20beak) 2e+02 true false -1.5e+02)
  (for _array_element (Variables|Default|GetALL%20Lokers)
    (Class|BPIGestionReparation|BreaktheObject(Message) _array_element self)))

(fn ConstructionScript)