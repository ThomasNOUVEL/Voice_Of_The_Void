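; BP_QuestObject is a breakable quest object for the Climatisation quest, using its Cube's material to show its state.
; On BeginPlay it caches BP_GestionHUD; Breakobject flags it broken and clears the material override.
; Interacting while broken asks the HUD to open WBP_ClimatisationQuest, passing itself as the quest object.
; Repareobject maps repair progress to one of four wood and bark materials, without resetting the broken flag.
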(event Custom|Break%20object
  (Variables|Default|SetBreak true)
  (Rendering|Material|SetMaterial (Variables|Default|GetCube) 0 0))

(event Custom|Repare%20object
  (params (Avancement :type Integer))
  (Rendering|Material|SetMaterial (Variables|Default|GetCube) 0 (Utilities|Select :Index Avancement :Option%200 "/Game/Materials/Bois_6_Mat.Bois_6_Mat" :Option%201 "/Game/Materials/Bois_4_Mat.Bois_4_Mat" :Option%202 "/Game/Materials/Bois_7_Mat.Bois_7_Mat" :Option%203 "/Game/Materials/Ecorce_Mat.Ecorce_Mat")))

(event EventBeginPlay
  (|CallParentFunction)
  (bind _returnvalue (Actor|GetActorOfClass "/Game/Blueprint/Widgets/BP_GestionHUD.BP_GestionHUD_C"))
  (Variables|Default|SetGestion%20HUD%20ref _returnvalue))

(event Collision|EventActorBeginOverlap
  (params (OtherActor :type Actor%20Object%20Reference))
  (|CallParentFunction OtherActor) ; This node is disabled and will not be called.\nDrag off pins to build functionality.
)

(event EventTick
  (params (DeltaSeconds :type Float%20%28single-precision%29))
  (|CallParentFunction DeltaSeconds) ; This node is disabled and will not be called.\nDrag off pins to build functionality.
)

(event EventInterract
  (params (First%20person%20ref :type BP%20First%20Person%20Character%20Object%20Reference))
  (Variables|Default|SetFirst%20Person%20Ref First%20person%20ref)
  (if (Variables|Default|GetBreak)
    (Default|Quest (Variables|Default|GetGestion%20HUD%20ref) "/Game/Blueprint/Widgets/WBP_ClimatisationQuest.WBP_ClimatisationQuest_C" self)))

(fn ConstructionScript
  (|CallParentFunction))