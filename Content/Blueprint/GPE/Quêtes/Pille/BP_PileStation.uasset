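; BP_PileStation is an interactable station the player takes a battery from or places one into.
; Interact, debounced by a half-second gate, swaps battery energy and hand state with the first-person character and toggles the battery mesh; a battery at energy 5 cannot be taken.
; A BP_BatteryCharge child actor shows the energy level, which BreaktheObject resets to zero.
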(event Custom|Delayed
  (Utilities|FlowControl|Delay 0.5)
  (Variables|Default|SetDelay true))

(event EventBeginPlay
  (|CallParentFunction)
  (bind _asbp_battery_charge (Utilities|Casting|CastToBP_BatteryCharge (Variables|/Script/Engine.ChildActorComponent|GetChildActor (Variables|Default|GetBP_BatteryCharge))))
  (bind _output_get (Variables|Default|SetAs%20BP%20Battery%20Charge _asbp_battery_charge))
  (Default|ChangeEnergyFeedBack _output_get (Variables|Default|GetBattery%20Energy)))

(event Collision|EventActorBeginOverlap
  (params (OtherActor :type Actor%20Object%20Reference))
  (|CallParentFunction OtherActor) ; This node is disabled and will not be called.\nDrag off pins to build functionality.
)

(event EventTick
  (params (DeltaSeconds :type Float%20%28single-precision%29))
  (|CallParentFunction DeltaSeconds) ; This node is disabled and will not be called.\nDrag off pins to build functionality.
)

(event EventInterract
  (params (First%20person%20ref :type BP%20First%20Person%20Character%20Object%20Reference))
  (Variables|Default|SetFirst%20Person%20Ref First%20person%20ref)
  (if (Variables|Default|GetDelay)
    (Variables|Default|SetDelay false)
    (CallFunction|Delayed)
    (if (Variables|Default|GetHave%20pile)
      (if (!= (Variables|Default|GetBattery%20Energy) 5)
        (if (or (== (Variables|/Game/FirstPerson/Blueprints/BP_FirstPersonCharacter.BP_FirstPersonCharacter_C|GetIn%20Hand (Variables|Default|GetFirst%20Person%20Ref)) 0) (== (Variables|/Game/FirstPerson/Blueprints/BP_FirstPersonCharacter.BP_FirstPersonCharacter_C|GetIn%20Hand (Variables|Default|GetFirst%20Person%20Ref)) 1))
          (Variables|/Game/FirstPerson/Blueprints/BP_FirstPersonCharacter.BP_FirstPersonCharacter_C|SetBattery%20Energy (Variables|Default|GetFirst%20Person%20Ref) (Variables|Default|GetBattery%20Energy))
          (Default|ChangeHandState (Variables|Default|GetFirst%20Person%20Ref) "NewEnumerator2")
          (Default|ChangeEnergyFeedBack (Variables|Default|GetAs%20BP%20Battery%20Charge) (Variables|Default|GetBattery%20Energy))
          (Variables|Default|SetHave%20pile false)
          (Rendering|SetVisibility (Variables|Default|GetBattery) false true)))
      (elif (== (Variables|/Game/FirstPerson/Blueprints/BP_FirstPersonCharacter.BP_FirstPersonCharacter_C|GetIn%20Hand (Variables|Default|GetFirst%20Person%20Ref)) 2)
        (Variables|Default|SetBattery%20Energy (Variables|/Game/FirstPerson/Blueprints/BP_FirstPersonCharacter.BP_FirstPersonCharacter_C|GetBattery%20Energy (Variables|Default|GetFirst%20Person%20Ref)))
        (Default|ChangeHandState (Variables|Default|GetFirst%20Person%20Ref) (Variables|/Game/FirstPerson/Blueprints/BP_FirstPersonCharacter.BP_FirstPersonCharacter_C|GetHave%20light (Variables|Default|GetFirst%20Person%20Ref)))
        (Default|ChangeEnergyFeedBack (Variables|Default|GetAs%20BP%20Battery%20Charge) (Variables|Default|GetBattery%20Energy))
        (Variables|Default|SetHave%20pile true)
        (Rendering|SetVisibility (Variables|Default|GetBattery) true true)))))

(event EventBreaktheObject
  (Variables|Default|SetBattery%20Energy 0)
  (Default|ChangeEnergyFeedBack (Variables|Default|GetAs%20BP%20Battery%20Charge) (Variables|Default|GetBattery%20Energy)))

(fn ConstructionScript
  (|CallParentFunction))