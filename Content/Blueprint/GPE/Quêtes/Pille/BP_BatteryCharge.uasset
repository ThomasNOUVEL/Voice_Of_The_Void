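; BP_BatteryCharge is a battery quest prop that displays an energy level on five LED meshes.
; Its Changeenergyfeedback event resets every LED to the screen material, then sets the on material on each LED up to the given Energy.
; A StopLoop flag limits the off material to the first LED above that level, leaving the remaining ones on the screen material.
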(event Custom|Change%20energy%20feed%20back
  (params (Energy :type Integer))
  (bind _led1 (Variables|Default|GetLed1))
  (Variables|Default|SetStop%20loop false)
  (Rendering|Material|SetMaterial (Variables|Default|GetLed5) 0 "/Game/Blueprint/GPE/Quêtes/Sincronisation/Mat_Screen.Mat_Screen")
  (for _index (range 1 5)
    (if (<= _index Energy)
      (Rendering|Material|SetMaterial (Utilities|Select :Index _index :Option%200 _led1 :Option%201 _led1 :Option%202 (Variables|Default|GetLed2) :Option%203 (Variables|Default|GetLed3) :Option%204 (Variables|Default|GetLed4) :Option%205 (Variables|Default|GetLed5)) 0 "/Game/Blueprint/GPE/Quêtes/Sincronisation/Mat_On.Mat_On")
      (elif (not (Variables|Default|GetStop%20loop))
        (Rendering|Material|SetMaterial (Utilities|Select :Index _index :Option%200 _led1 :Option%201 _led1 :Option%202 (Variables|Default|GetLed2) :Option%203 (Variables|Default|GetLed3) :Option%204 (Variables|Default|GetLed4) :Option%205 (Variables|Default|GetLed5)) 0 "/Game/Blueprint/GPE/Quêtes/Sincronisation/Mat_Off.Mat_Off")
        (Variables|Default|SetStop%20loop true)))))

(event EventBeginPlay)

(event Collision|EventActorBeginOverlap
  (params (OtherActor :type Actor%20Object%20Reference)))

(event EventTick
  (params (DeltaSeconds :type Float%20%28single-precision%29)))

(fn ConstructionScript)