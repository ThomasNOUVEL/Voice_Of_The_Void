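; Rotatable nut (écrou) puzzle piece for the wiring (Cablage) quest, reporting to a manager actor.
; Each allowed interaction plays a timeline turning the base 90 degrees through four states, with Delay blocking input during animation.
; Reaching the target state extends the ObjectifDent tooth via a second timeline, then notifies the manager.
; Interacting again reverses that timeline, then rotates onward and tells the manager the chain is broken.
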(event Custom|TableauCablageRef
  (params (Actor%20Next%20To :type BP%20Tableau%20Cablage%20Object%20Reference))
  (Variables|Default|SetGestionnaire%20ref Actor%20Next%20To))

(event Custom|Out%20Good%20state
  (bind _objectif_dent (Variables|Default|GetObjectif%20Dent))
  (bind _relativerotation (Variables|/Script/Engine.SceneComponent|GetRelativeRotation _objectif_dent))
  (Variables|Default|SetBool%20Good%20state false)
  (bind (_direction _float) (Timeline|Good%20State ReverseFromEnd)
    (:Update
      (Transformation|SetRelativeTransform _objectif_dent (Math|Transform|Lerp(Transform) (Math|Transform|MakeTransform "113.137086,113.137084,0.000000" _relativerotation "1.843750,-0.640000,0.320000") (Math|Transform|MakeTransform "339.411257,339.411253,0.000000" _relativerotation "11.000000,-0.640000,0.320000") _float) false false))
    (:Finished
      (switch Utilities|FlowControl|Switch|SwitchonETimelineDirection _direction
        (:Forward
          (Variables|Default|SetDelay true)
          (Default|GoodPositionEcrous (Variables|Default|GetGestionnaire%20ref) self)
          (Variables|Default|SetBool%20Good%20state true))
        (:Backward
          (CallFunction|Rotation)
          (Default|BreaktheChaine (Variables|Default|GetGestionnaire%20ref) self)
          (Variables|Default|SetBool%20Good%20state false))))))

(event Custom|Rotation
  (bind _float (Timeline|RotationEcrous PlayFromStart)
    (:Update
      (Transformation|SetRelativeRotation (Variables|Default|GetBase) (Math|Rotator|Lerp(Rotator) (Math|Rotator|MakeRotator 9e+01 (Utilities|Select :Index (Variables|Default|GetRotationState) :Option%200 0.0 :Option%201 9e+01 :Option%202 1.8e+02 :Option%203 2.7e+02) 0.0) (Math|Rotator|MakeRotator 9e+01 (+ (Utilities|Select :Index (Variables|Default|GetRotationState) :Option%200 0.0 :Option%201 9e+01 :Option%202 1.8e+02 :Option%203 2.7e+02) 9e+01) 0.0) _float) false false)
      (bind _result (Math|Float|NegateFloat (.Pitch (Math|Rotator|BreakRotator (Math|Rotator|Lerp(Rotator) (Math|Rotator|MakeRotator 9e+01 (Utilities|Select :Index (Variables|Default|GetRotationState) :Option%200 0.0 :Option%201 9e+01 :Option%202 1.8e+02 :Option%203 2.7e+02) 0.0) (Math|Rotator|MakeRotator 9e+01 (+ (Utilities|Select :Index (Variables|Default|GetRotationState) :Option%200 0.0 :Option%201 9e+01 :Option%202 1.8e+02 :Option%203 2.7e+02) 9e+01) 0.0) _float))))
        (:%20%20
          (Transformation|SetRelativeRotation (Variables|Default|GetObjectif) (Math|Rotator|MakeRotator (.Roll (Math|Rotator|BreakRotator (Math|Rotator|Lerp(Rotator) (Math|Rotator|MakeRotator 9e+01 (Utilities|Select :Index (Variables|Default|GetRotationState) :Option%200 0.0 :Option%201 9e+01 :Option%202 1.8e+02 :Option%203 2.7e+02) 0.0) (Math|Rotator|MakeRotator 9e+01 (+ (Utilities|Select :Index (Variables|Default|GetRotationState) :Option%200 0.0 :Option%201 9e+01 :Option%202 1.8e+02 :Option%203 2.7e+02) 9e+01) 0.0) _float))) _result 0.0) false false))))
    (:Finished
      (Variables|Default|SetRotationState (Utilities|Select :Index (Variables|Default|GetRotationState) :Option%200 1 :Option%201 2 :Option%202 3 :Option%203 0))
      (if (== (Variables|Default|GetRotationState) (Variables|Default|GetRotationObjectif))
        (CallFunction|InGoodState)
        (else
          (Variables|Default|SetDelay true))))))

(event Custom|In%20good%20state
  (bind _objectif_dent (Variables|Default|GetObjectif%20Dent))
  (bind _relativerotation (Variables|/Script/Engine.SceneComponent|GetRelativeRotation _objectif_dent))
  (Variables|Default|SetBool%20Good%20state true)
  (bind (_direction _float) (Timeline|Good%20State PlayFromStart)
    (:Update
      (Transformation|SetRelativeTransform _objectif_dent (Math|Transform|Lerp(Transform) (Math|Transform|MakeTransform "113.137086,113.137084,0.000000" _relativerotation "1.843750,-0.640000,0.320000") (Math|Transform|MakeTransform "339.411257,339.411253,0.000000" _relativerotation "11.000000,-0.640000,0.320000") _float) false false))
    (:Finished
      (switch Utilities|FlowControl|Switch|SwitchonETimelineDirection _direction
        (:Forward
          (Variables|Default|SetDelay true)
          (Default|GoodPositionEcrous (Variables|Default|GetGestionnaire%20ref) self)
          (Variables|Default|SetBool%20Good%20state true))
        (:Backward
          (CallFunction|Rotation)
          (Default|BreaktheChaine (Variables|Default|GetGestionnaire%20ref) self)
          (Variables|Default|SetBool%20Good%20state false))))))

(event EventBeginPlay
  (|CallParentFunction) ; This node is disabled and will not be called.\nDrag off pins to build functionality.
)

(event Collision|EventActorBeginOverlap
  (params (OtherActor :type Actor%20Object%20Reference))
  (|CallParentFunction OtherActor) ; This node is disabled and will not be called.\nDrag off pins to build functionality.
)

(event EventTick
  (params (DeltaSeconds :type Float%20%28single-precision%29))
  (|CallParentFunction DeltaSeconds) ; This node is disabled and will not be called.\nDrag off pins to build functionality.
)

(event EventInterract
  (params (First%20person%20ref :type BP%20First%20Person%20Character%20Object%20Reference))
  (if (Variables|Default|GetCan%20interract)
    (if (Variables|Default|GetDelay)
      (Variables|Default|SetDelay false)
      (if (Variables|Default|GetBool%20Good%20state)
        (CallFunction|OutGoodState)
        (else
          (CallFunction|Rotation))))))

(fn ConstructionScript
  (|CallParentFunction))