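; BP_GestionTableau manages a tableau (panel) for the wiring quest, swapping it to a broken state and reporting its repair.
; On play it replaces its placeholder with a spawned BP_FlipFlopTableau and hands it a self-reference.
; BreaktheObject stores the calling quest manager, then after a short delay destroys and respawns the tableau with BreakSide applied.
; Questfinish notifies that manager through QuestRepared.
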(event Custom|Quest%20finish
  (Default|QuestRepared (Variables|Default|GetBP%20Gestion%20Quete) self))

(event EventBreaktheObject
  (params (BP_GestionQuete :type BP%20Gestion%20Quete%20Object%20Reference))
  (Variables|Default|SetBP%20Gestion%20Quete BP_GestionQuete)
  (Variables|Default|SetBreak true)
  (Utilities|FlowControl|Delay 0.2)
  (Actor|DestroyActor (Variables|Default|GetFlip%20Flop%20ref))
  (bind _returnvalue (Game|SpawnActorfromClass "/Game/Blueprint/GPE/Quêtes/Cablage/BP_FlipFlopTableau.BP_FlipFlopTableau_C" (Transformation|GetActorTransform) "Undefined" "MultiplyWithRoot" 0 0))
  (Variables|Default|SetFlip%20Flop%20ref _returnvalue)
  (Default|BreakSide (Variables|Default|GetFlip%20Flop%20ref))
  (Default|GestionTabRef (Variables|Default|GetFlip%20Flop%20ref) self))

(event EventBeginPlay
  (Components|DestroyComponent (Variables|Default|GetBP_FlipFlopTableau))
  (bind _returnvalue (Game|SpawnActorfromClass "/Game/Blueprint/GPE/Quêtes/Cablage/BP_FlipFlopTableau.BP_FlipFlopTableau_C" (Transformation|GetActorTransform) "Undefined" "MultiplyWithRoot" 0 0))
  (bind _output_get (Variables|Default|SetFlip%20Flop%20ref _returnvalue))
  (Default|GestionTabRef _output_get self))

(fn ConstructionScript)