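; BP_SecurityCode is a security code display that generates a random four-digit code and shows it on its TextRender component.
; On BeginPlay it builds the code from four random non-zero digits, each scaled by its decimal place, and stores the sum in SecurityCode.
; The Refreshcode event reruns the same generation and display chain, and GetSecurityCode exposes the current value to other Blueprints.
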(event Custom|Refresh%20code
  (bind _returnvalue (Math|Random|RandomIntegerinRange 1 9))
  (bind _returnvalue_2 (* _returnvalue 10))
  (bind _returnvalue_3 (* _returnvalue_2 10))
  (Variables|Default|SetSecurityCode _returnvalue)
  (Variables|Default|SetSecurityCode (+ (Variables|Default|GetSecurityCode) _returnvalue_2))
  (Variables|Default|SetSecurityCode (+ (Variables|Default|GetSecurityCode) _returnvalue_3))
  (Variables|Default|SetSecurityCode (+ (Variables|Default|GetSecurityCode) (* _returnvalue_3 10)))
  (Rendering|Components|TextRender|SetText (Variables|Default|GetTextRender) (Utilities|Text|ToText(String) (Utilities|String|ToString(Integer) (Variables|Default|GetSecurityCode)))))

(event EventBeginPlay
  (bind _returnvalue (Math|Random|RandomIntegerinRange 1 9))
  (bind _returnvalue_2 (* _returnvalue 10))
  (bind _returnvalue_3 (* _returnvalue_2 10))
  (Variables|Default|SetSecurityCode _returnvalue)
  (Variables|Default|SetSecurityCode (+ (Variables|Default|GetSecurityCode) _returnvalue_2))
  (Variables|Default|SetSecurityCode (+ (Variables|Default|GetSecurityCode) _returnvalue_3))
  (Variables|Default|SetSecurityCode (+ (Variables|Default|GetSecurityCode) (* _returnvalue_3 10)))
  (Rendering|Components|TextRender|SetText (Variables|Default|GetTextRender) (Utilities|Text|ToText(String) (Utilities|String|ToString(Integer) (Variables|Default|GetSecurityCode)))))

(fn ConstructionScript)

(fn GetSecurityCode
  (return (Variables|Default|GetSecurityCode)))