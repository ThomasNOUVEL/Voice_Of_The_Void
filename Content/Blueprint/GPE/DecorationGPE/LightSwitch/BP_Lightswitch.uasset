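; Interactable light switch decoration that toggles a set of referenced lights when the player interacts with it.
; Each accepted interaction flips the on/off state, rotates the switch mesh and adds an audio component, with a short delay flag blocking repeat presses.
; The referenced lights change intensity to match the state only when the Electricity flag is set, so an unpowered switch still flips.
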(event Custom|switch%20the%20light
  (bind _switch (Variables|Default|GetSwitch))
  (if (Variables|Default|GetOn/Off)
    (Variables|Default|SetOn/Off false)
    (Transformation|SetRelativeRotation _switch "30.000000,89.999999,0.000000" false false)
    (AddComponent|AddAudioComponent false)
    (else
      (Variables|Default|SetOn/Off true)
      (Transformation|SetRelativeRotation _switch "-30.000000,89.999999,0.000000" false false)
      (AddComponent|AddAudioComponent false)))
  (Utilities|FlowControl|Delay 0.4)
  (Variables|Default|Setdelay true))

(event EventBeginPlay
  (|CallParentFunction) ; This node is disabled and will not be called.\nDrag off pins to build functionality.
)

(event Collision|EventActorBeginOverlap
  (params (OtherActor :type Actor%20Object%20Reference))
  (|CallParentFunction OtherActor) ; This node is disabled and will not be called.\nDrag off pins to build functionality.
)

(event EventTick
  (params (DeltaSeconds :type Float%20%28single-precision%29))
  (|CallParentFunction DeltaSeconds) ; This node is disabled and will not be called.\nDrag off pins to build functionality.
)

(event EventInterract
  (params (First%20person%20ref :type BP%20First%20Person%20Character%20Object%20Reference))
  (Variables|Default|SetFirst%20Person%20Ref First%20person%20ref)
  (if (Variables|Default|Getdelay)
    (Variables|Default|Setdelay false)
    (CallFunction|SwitchtheLight)
    (if (Variables|Default|GetElectricity)
      (for _array_element (Variables|Default|GetArray%20Light%20Refs)
        (Rendering|Components|Light|SetIntensity (Variables|/Script/Engine.Light|GetLightComponent _array_element) (Math|Float|SelectFloat 1e+02 0.0 (Variables|Default|GetOn/Off)))))))

(fn ConstructionScript
  (|CallParentFunction))