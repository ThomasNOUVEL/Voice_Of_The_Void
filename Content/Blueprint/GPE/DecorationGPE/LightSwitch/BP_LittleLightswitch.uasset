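; BP_LittleLightswitch is an interactable secondary light switch that works as a remote for a linked main switch.
; On BeginPlay it registers with MaineSwitch; interacting flips OnOff, rotates the switch mesh, plays audio and reports the state to MaineSwitch, with a short Delay-flag cooldown.
; OtherswitchUp sets state and rotation without sound or reporting back.
; The Power on/off functions are empty, with disconnected light-intensity logic.
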(event Custom|switch%20the%20light
  (bind _switch (Variables|Default|GetSwitch))
  (if (Variables|Default|GetOn%20Off)
    (Variables|Default|SetOn%20Off false)
    (Transformation|SetRelativeRotation _switch "30.000000,89.999999,0.000000" false false)
    (AddComponent|AddAudioComponent false)
    (else
      (Variables|Default|SetOn%20Off true)
      (Transformation|SetRelativeRotation _switch "-30.000000,89.999999,0.000000" false false)
      (AddComponent|AddAudioComponent false)))
  (Default|MaineSwitchChange (Variables|Default|GetMaine%20switch) (Variables|Default|GetOn%20Off))
  (Utilities|FlowControl|Delay 0.5)
  (Variables|Default|Setdelay true))

(event Custom|Other%20switch%20Up
  (params (Condition :type Boolean))
  (bind _switch (Variables|Default|GetSwitch))
  (if Condition
    (Variables|Default|SetOn%20Off true)
    (Transformation|SetRelativeRotation _switch "-30.000000,89.999999,0.000000" false false)
    (else
      (Variables|Default|SetOn%20Off false)
      (Transformation|SetRelativeRotation _switch "30.000000,89.999999,0.000000" false false))))

(event EventBeginPlay
  (|CallParentFunction)
  (Utilities|Array|Add (Variables|/Game/Blueprint/GPE/DecorationGPE/LightSwitch/BP_ManeLightswitch.BP_ManeLightswitch_C|GetOther%20switch (Variables|Default|GetMaine%20switch)) self))

(event Collision|EventActorBeginOverlap
  (params (OtherActor :type Actor%20Object%20Reference))
  (|CallParentFunction OtherActor) ; This node is disabled and will not be called.\nDrag off pins to build functionality.
)

(event EventTick
  (params (DeltaSeconds :type Float%20%28single-precision%29))
  (|CallParentFunction DeltaSeconds) ; This node is disabled and will not be called.\nDrag off pins to build functionality.
)

(event EventInterract
  (params (First%20person%20ref :type BP%20First%20Person%20Character%20Object%20Reference))
  (Variables|Default|SetFirst%20Person%20Ref First%20person%20ref)
  (if (Variables|Default|Getdelay)
    (Variables|Default|Setdelay false)
    (CallFunction|SwitchtheLight)))

(fn ConstructionScript
  (|CallParentFunction))

(fn PowerOff)

(fn Poweron)