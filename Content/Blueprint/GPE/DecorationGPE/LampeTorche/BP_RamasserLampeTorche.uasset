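; Flashlight pickup actor that gives the first-person character a torch when interacted with.
; Its Interract event stores the player reference and sets that character's HaveLight state.
; If the character's InHand state is at its first value, it also calls ChangeHandState to switch the hand state, then destroys itself.
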(event EventBeginPlay
  (|CallParentFunction) ; This node is disabled and will not be called.\nDrag off pins to build functionality.
)

(event Collision|EventActorBeginOverlap
  (params (OtherActor :type Actor%20Object%20Reference))
  (|CallParentFunction OtherActor) ; This node is disabled and will not be called.\nDrag off pins to build functionality.
)

(event EventTick
  (params (DeltaSeconds :type Float%20%28single-precision%29))
  (|CallParentFunction DeltaSeconds) ; This node is disabled and will not be called.\nDrag off pins to build functionality.
)

(event EventInterract
  (params (First%20person%20ref :type BP%20First%20Person%20Character%20Object%20Reference))
  (Variables|Default|SetFirst%20Person%20Ref First%20person%20ref)
  (Variables|/Game/FirstPerson/Blueprints/BP_FirstPersonCharacter.BP_FirstPersonCharacter_C|SetHave%20light (Variables|Default|GetFirst%20Person%20Ref) "NewEnumerator1")
  (if (== (Variables|/Game/FirstPerson/Blueprints/BP_FirstPersonCharacter.BP_FirstPersonCharacter_C|GetIn%20Hand (Variables|Default|GetFirst%20Person%20Ref)) 0)
    (Default|ChangeHandState (Variables|Default|GetFirst%20Person%20Ref) "NewEnumerator1"))
  (Actor|DestroyActor))

(fn ConstructionScript
  (|CallParentFunction))