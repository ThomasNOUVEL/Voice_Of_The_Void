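; BP_OfficeGlobe is a decorative office globe that spins when interacted with.
; The Interract event plays the Rotation timeline, which lerps the Sphere's yaw from its current relative rotation to 500 degrees further.
; The same timeline lowers the pitch and volume of the RollingGlobe sound as it progresses, stopping it below a threshold or when the timeline finishes.
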(event Custom|Play%20sound
  (bind _rolling_globe (Variables|Default|GetRolling_Globe))
  (Utilities|IsValid _rolling_globe
    (:Is%20Valid
      (if (not (Audio|Components|Audio|IsPlaying _rolling_globe))
        (Audio|Components|Audio|Play (Variables|Default|GetRolling_Globe) 0.0 :!label _label)))
    (:Is%20Not%20Valid
      (goto _label))))

(event EventBeginPlay
  (|CallParentFunction)
  (Audio|Components|Audio|Stop (Variables|Default|GetRolling_Globe)))

(event Collision|EventActorBeginOverlap
  (params (OtherActor :type Actor%20Object%20Reference))
  (|CallParentFunction OtherActor) ; This node is disabled and will not be called.\nDrag off pins to build functionality.
)

(event EventTick
  (params (DeltaSeconds :type Float%20%28single-precision%29))
  (|CallParentFunction DeltaSeconds) ; This node is disabled and will not be called.\nDrag off pins to build functionality.
)

(event EventInterract
  (params (First%20person%20ref :type BP%20First%20Person%20Character%20Object%20Reference))
  (bind _rolling_globe (Variables|Default|GetRolling_Globe))
  (Variables|Default|SetFirst%20Person%20Ref First%20person%20ref)
  (Variables|Default|SetStart%20rotation (Variables|/Script/Engine.SceneComponent|GetRelativeRotation (Variables|Default|GetSphere)))
  (CallFunction|PlaySound)
  (bind _float (Timeline|Rotation PlayFromStart)
    (:Update
      (Transformation|SetRelativeRotation (Variables|Default|GetSphere) (Math|Rotator|Lerp(Rotator) (Variables|Default|GetStart%20rotation) (Math|Rotator|MakeRotator (.Roll (Math|Rotator|BreakRotator (Variables|Default|GetStart%20rotation))) (.Pitch (Math|Rotator|BreakRotator (Variables|Default|GetStart%20rotation))) (+ (.Yaw (Math|Rotator|BreakRotator (Variables|Default|GetStart%20rotation))) 5e+02)) _float) false false)
      (if (< (- 1.0 (/ _float 2.0)) 0.53)
        (Audio|Components|Audio|Stop _rolling_globe)
        (else
          (Audio|Components|Audio|SetPitchMultiplier _rolling_globe (- 1.0 (/ _float 2.0)))
          (Audio|Components|Audio|SetVolumeMultiplier _rolling_globe (- 1.0 (/ _float 2.0)) :!class /Script/Engine.AudioComponent))))
    (:Finished
      (Audio|Components|Audio|Stop (Variables|Default|GetRolling_Globe)))))

(fn ConstructionScript
  (|CallParentFunction))