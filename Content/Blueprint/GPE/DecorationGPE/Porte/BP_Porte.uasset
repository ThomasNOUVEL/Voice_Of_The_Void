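; BP_Porte is an interactable door that opens and closes as either a sliding or classic hinged door.
; Interract does nothing while Loker is set or a move is running, with Delay acting as the re-trigger gate.
; SliderDoor picks a timeline that slides or rotates the Charniere component, with OppenDirectionRL setting the swing side.
; Timelines play forward or reverse according to Oppen, which flips on completion.
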(event EventBeginPlay
  (|CallParentFunction) ; This node is disabled and will not be called.\nDrag off pins to build functionality.
)

(event Collision|EventActorBeginOverlap
  (params (OtherActor :type Actor%20Object%20Reference))
  (|CallParentFunction OtherActor) ; This node is disabled and will not be called.\nDrag off pins to build functionality.
)

(event EventTick
  (params (DeltaSeconds :type Float%20%28single-precision%29))
  (|CallParentFunction DeltaSeconds) ; This node is disabled and will not be called.\nDrag off pins to build functionality.
)

(event EventInterract
  (params (First%20person%20ref :type BP%20First%20Person%20Character%20Object%20Reference))
  (bind _returnvalue (Math|Float|MakeLiteralFloat 1e+02))
  (if (not (Variables|Default|GetLoker))
    (if (Variables|Default|GetDelay)
      (Variables|Default|SetDelay false)
      (if (Variables|Default|GetSliderDoor)
        ;[0.15 0.15 0.15 0.5] Slider door
        (if (Variables|Default|GetOppen)
          (bind _float (Timeline|Timeline_0 ReverseFromEnd)
            (:Update
              (Transformation|SetRelativeLocation (Variables|Default|GetCharniere) (Math|Vector|Lerp(Vector) "-57.000000,0.000000,-12.000000" "-170.000000,0.000000,-12.000000" _float) false false))
            (:Finished
              (Variables|Default|SetOppen (not (Variables|Default|GetOppen)))
              (Variables|Default|SetDelay true)))
          (else
            (Timeline|Timeline_0 PlayFromStart)))
        (else
          ;[0.15 0.15 0.15 0.5] Clasic door
          (if (Variables|Default|GetOppen)
            (bind _float_2 (Timeline|Timeline ReverseFromEnd)
              (:Update
                (Transformation|SetRelativeRotation (Variables|Default|GetCharniere) (Math|Rotator|Lerp(Rotator) "0, 0, 0" (Math|Rotator|MakeRotator 0.0 0.0 (select (Variables|Default|GetOppen%20direction%20R%20L) _returnvalue (* _returnvalue -1.0))) _float_2) false false))
              (:Finished
                (Variables|Default|SetOppen (not (Variables|Default|GetOppen)))
                (Variables|Default|SetDelay true)))
            (else
              (Timeline|Timeline PlayFromStart))))))))

(fn ConstructionScript
  (|CallParentFunction))