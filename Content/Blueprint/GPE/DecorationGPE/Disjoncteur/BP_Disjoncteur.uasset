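; Interactable circuit breaker that switches power for every BP_Lightswitch in the level and trips when too many lights are on.
; Interaction toggles power with a short click cooldown, then SetPower flips the lever, swaps the LED material, adds audio and notifies all light switches.
; NewSwitch keeps a count of switched-on lights, reset on power-up, and cuts power after a brief delay once it reaches the limit.
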(event Custom|Click%20Delay
  ;[0.15 0.15 0.15 0.5] Interraction
  (Variables|Default|SetDelay false)
  (Utilities|FlowControl|Delay 0.5)
  (Variables|Default|SetDelay true))

(event Custom|Set%20Power
  (bind _led_disjoncteur (Variables|Default|GetLed%20Disjoncteur))
  ;[0.15 0.15 0.15 0.5] Set Map Power
  (Transformation|SetRelativeRotation (Variables|Default|GetSwitch) (select (Variables|Default|GetPower%20On%20off) "-30.000000,0.000000,0.000000" "30.000000,0.000000,0.000000") false false)
  (if (Variables|Default|GetPower%20On%20off)
    (AddComponent|AddAudioComponent false)
    (Rendering|Material|SetMaterial _led_disjoncteur 0 "/Game/Blueprint/GPE/Quêtes/Sincronisation/Mat_On.Mat_On")
    (Variables|Default|SetLightPower 0)
    (else
      (AddComponent|AddAudioComponent false)
      (Rendering|Material|SetMaterial _led_disjoncteur 0 "/Game/Blueprint/GPE/Quêtes/Sincronisation/Mat_Off.Mat_Off")))
  (bind _outactors (Actor|GetAllActorsOfClass "/Game/Blueprint/GPE/DecorationGPE/LightSwitch/BP_Lightswitch.BP_Lightswitch_C"))
  (for _array_element _outactors
    (if (Variables|Default|GetPower%20On%20off)
      (Default|Poweron _array_element)
      (else
        (Default|PowerOff _array_element)))))

(event Custom|New%20Switch
  (params (On%20Off :type Boolean))
  (bind _lightpower (Variables|Default|GetLightPower))
  ;[0.15 0.15 0.15 0.5] Count Of Switch On
  (if On%20Off
    (Math|Integer|IncrementInt _lightpower
      (:%20%20
        _))
    (else
      (Math|Integer|DecrementInt _lightpower
        (:%20%20
          _))))
  (Utilities|FlowControl|Delay 0.2)
  (if (>= (Variables|Default|GetLightPower) 4)
    (Variables|Default|SetPower%20On%20off false)
    (CallFunction|SetPower)))

(event EventBeginPlay
  (|CallParentFunction) ; This node is disabled and will not be called.\nDrag off pins to build functionality.
)

(event Collision|EventActorBeginOverlap
  (params (OtherActor :type Actor%20Object%20Reference))
  (|CallParentFunction OtherActor) ; This node is disabled and will not be called.\nDrag off pins to build functionality.
)

(event EventTick
  (params (DeltaSeconds :type Float%20%28single-precision%29))
  (|CallParentFunction DeltaSeconds) ; This node is disabled and will not be called.\nDrag off pins to build functionality.
)

(event EventInterract
  (params (First%20person%20ref :type BP%20First%20Person%20Character%20Object%20Reference))
  ;[0.15 0.15 0.15 0.5] Interraction
  (Variables|Default|SetFirst%20Person%20Ref First%20person%20ref)
  (if (Variables|Default|GetDelay)
    (CallFunction|ClickDelay)
    (Variables|Default|SetPower%20On%20off (not (Variables|Default|GetPower%20On%20off)))
    (CallFunction|SetPower)))

(fn ConstructionScript
  (|CallParentFunction))