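; BP_DisjoncteurDoor is an interactable circuit breaker door that the player swings open and closed.
; Each Interract stores the first-person reference and flips between opening and closing, playing the matching sound.
; The Oppening timeline, played forward or in reverse, lerps the Pivot's rotation to swing the door.
; A Delay flag blocks new interactions until the timeline finishes.
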(event EventBeginPlay
  (|CallParentFunction)
  (Audio|Components|Audio|Stop (Variables|Default|GetOppen_disjoncteur)))

(event Collision|EventActorBeginOverlap
  (params (OtherActor :type Actor%20Object%20Reference))
  (|CallParentFunction OtherActor) ; This node is disabled and will not be called.\nDrag off pins to build functionality.
)

(event EventTick
  (params (DeltaSeconds :type Float%20%28single-precision%29))
  (|CallParentFunction DeltaSeconds) ; This node is disabled and will not be called.\nDrag off pins to build functionality.
)

(event EventInterract
  (params (First%20person%20ref :type BP%20First%20Person%20Character%20Object%20Reference))
  (bind _oppen_disjoncteur (Variables|Default|GetOppen_disjoncteur))
  (Variables|Default|SetFirst%20Person%20Ref First%20person%20ref)
  (if (Variables|Default|GetDelay)
    (Variables|Default|SetDelay false)
    (Utilities|FlowControl|FlipFlop
      (:A
        (Audio|Components|Audio|SetSound _oppen_disjoncteur "/Game/Blueprint/GPE/DecorationGPE/Disjoncteur/Oppen_disjoncteur.Oppen_disjoncteur")
        (Audio|Components|Audio|Play _oppen_disjoncteur 0.0)
        (bind _float (Timeline|Oppening PlayFromStart)
          (:Update
            (Transformation|SetRelativeRotation (Variables|Default|GetPivot) (Math|Rotator|Lerp(Rotator) "0, 0, 0" "0.000000,170.000000,0.000000" _float) false false))
          (:Finished
            (Variables|Default|SetDelay true))))
      (:B
        (Audio|Components|Audio|SetSound _oppen_disjoncteur "/Game/Blueprint/GPE/DecorationGPE/Disjoncteur/Close_Disjoncteur.Close_Disjoncteur")
        (Audio|Components|Audio|Play _oppen_disjoncteur 0.0)
        (Timeline|Oppening ReverseFromEnd)))))

(fn ConstructionScript
  (|CallParentFunction))