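; Interactable desk drawer that slides open and shut when the player interacts with it.
; Interract ignores input while moving, toggles the Close state, and swaps in the matching open or close sound.
; The Ouverture timeline, played forward or reversed, lerps the drawer's relative location and clears the moving lock when finished.
; A FlipFlop alternates the TextRender between two joke strings on successive openings.
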(event EventBeginPlay
  (|CallParentFunction)
  (Audio|Components|Audio|Stop (Variables|Default|GetTiroire%20soud)))

(event Collision|EventActorBeginOverlap
  (params (OtherActor :type Actor%20Object%20Reference))
  (|CallParentFunction OtherActor) ; This node is disabled and will not be called.\nDrag off pins to build functionality.
)

(event EventTick
  (params (DeltaSeconds :type Float%20%28single-precision%29))
  (|CallParentFunction DeltaSeconds) ; This node is disabled and will not be called.\nDrag off pins to build functionality.
)

(event EventInterract
  (params (First%20person%20ref :type BP%20First%20Person%20Character%20Object%20Reference))
  (bind _textrender (Variables|Default|GetTextRender))
  (bind _tiroire_soud (Variables|Default|GetTiroire%20soud))
  (Variables|Default|SetFirst%20Person%20Ref First%20person%20ref)
  (if (not (Variables|Default|GetIs%20mooving))
    (Variables|Default|SetIs%20mooving true)
    (if (Variables|Default|GetClose)
      (Variables|Default|SetClose false)
      (Audio|Components|Audio|SetSound _tiroire_soud "/Game/Blueprint/GPE/DecorationGPE/TiroireDesktop/TiroireOppenSound.TiroireOppenSound")
      (Audio|Components|Audio|Play _tiroire_soud 0.15)
      (Utilities|FlowControl|FlipFlop
        (:A
          (Rendering|Components|TextRender|SetText _textrender (Utilities|Text|MakeLiteralText "Caca"))
          (bind _float (Timeline|Ouverture PlayFromStart)
            (:Update
              (Transformation|SetRelativeLocation (Variables|Default|GetTiroire) (Math|Vector|Lerp(Vector) "0, 0, 0" "35.000000,0.000000,0.000000" _float) false false))
            (:Finished
              (Variables|Default|SetIs%20mooving false))))
        (:B
          (Rendering|Components|TextRender|SetText _textrender (Utilities|Text|MakeLiteralText "67"))
          (Timeline|Ouverture PlayFromStart)))
      (else
        (Variables|Default|SetClose true)
        (Audio|Components|Audio|SetSound _tiroire_soud "/Game/Blueprint/GPE/DecorationGPE/TiroireDesktop/TiroireCloseSound.TiroireCloseSound")
        (Audio|Components|Audio|Play _tiroire_soud 0.1)
        (Timeline|Ouverture ReverseFromEnd)))))

(fn ConstructionScript
  (|CallParentFunction))