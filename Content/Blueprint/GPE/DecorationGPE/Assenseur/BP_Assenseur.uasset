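; Elevator actor that travels between stages in EtageTabRef and opens or closes the door at each stop.
; Gotostage closes the current door, waits briefly, then ChangeStage recursively moves the car one stage at a time with a Timeline lerp.
; Play rate scales inversely with the distance between stages to keep speed constant.
; On arrival it opens the door, waits, clears Mooving and notifies four child-actor buttons.
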(event Custom|Go%20to%20stage
  (params (What%20stage :type Integer))
  (bind _stage (Variables|Default|GetStage))
  ;[0.15 0.15 0.15 0.5] Where we need to go
  (Variables|Default|SetStage%20to%20go What%20stage)
  (if (not (== What%20stage _stage))
    (Default|ClosetheDoor (.Value (Utilities|Map|Find (Variables|Default|GetEtage%20tab%20ref) _stage)))
    (Variables|Default|SetMooving true)
    (Utilities|FlowControl|Delay 1.5)
    (Variables|Default|SetUp%20Down (> (Variables|Default|GetStage%20to%20go) (Variables|Default|GetStage)))
    (CallFunction|ChangeStage)))

(event Custom|Change%20Stage
  ;[0.15 0.15 0.15 0.5] Change stage
  (if (== (Variables|Default|GetStage%20to%20go) (Variables|Default|GetStage))
    ;;[0.2439 0.5417 0.2172] Finish
    (Default|OppentheDoor (.Value (Utilities|Map|Find (Variables|Default|GetEtage%20tab%20ref) (Variables|Default|GetStage))))
    (Utilities|FlowControl|Delay 2.5)
    (Variables|Default|SetMooving false)
    (for _index (range 0 3)
      (Default|Arrived (.AsBP%20Asssenseur%20Button (Utilities|Casting|CastToBP_AsssenseurButton (Variables|/Script/Engine.ChildActorComponent|GetChildActor (Utilities|Select :Index _index :Option%200 (Variables|Default|GetBP_AsssenseurButton3) :Option%201 (Variables|Default|GetBP_AsssenseurButton2) :Option%202 (Variables|Default|GetBP_AsssenseurButton) :Option%203 (Variables|Default|GetBP_AsssenseurButton1)))))))
    (else
      ;;[0.15 0.15 0.15 0.5] set stage
      (Variables|Default|SetStage (+ (Variables|Default|GetStage) (Math|Integer|SelectInt 1 -1 (Variables|Default|GetUp%20Down))))
      ;;[0.2116 0.2604 0.3906] Calculate movement speed by distance
      (Components|Timeline|SetPlayRate (Variables|Default|GetTimeline) (/ 1.0 (/ (Math|Vector|Distance(Vector) (Transformation|GetActorLocation (.Value (Utilities|Map|Find (Variables|Default|GetEtage%20tab%20ref) (+ (Variables|Default|GetStage) (Math|Integer|SelectInt -1 1 (Variables|Default|GetUp%20Down)))))) (Transformation|GetActorLocation (.Value (Utilities|Map|Find (Variables|Default|GetEtage%20tab%20ref) (Variables|Default|GetStage))))) 1e+02)))
      ;;[0.7391 0.6342 0.2946] Moovement
      (bind _float (Timeline|Timeline PlayFromStart)
        (:Update
          (Transformation|SetActorLocation (Math|Vector|Lerp(Vector) (Transformation|GetActorLocation (.Value (Utilities|Map|Find (Variables|Default|GetEtage%20tab%20ref) (+ (Variables|Default|GetStage) (Math|Integer|SelectInt -1 1 (Variables|Default|GetUp%20Down)))))) (Transformation|GetActorLocation (.Value (Utilities|Map|Find (Variables|Default|GetEtage%20tab%20ref) (Variables|Default|GetStage)))) _float) false false))
        (:Finished
          (CallFunction|ChangeStage))))))

(event EventBeginPlay
  (Default|OppentheDoor (.Value (Utilities|Map|Find (Variables|Default|GetEtage%20tab%20ref) (Variables|Default|GetStage)))))

(fn ConstructionScript)