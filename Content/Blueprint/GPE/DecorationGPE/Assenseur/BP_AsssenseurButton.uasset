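; BP_AsssenseurButton is an elevator button that sends BP_Assenseur to the floor given by its Number.
; On BeginPlay it displays that number on a text render and finds the elevator with GetActorOfClass.
; Interract calls GoToStage and switches the cube to Mat_On, only if the elevator is idle and on another stage.
; The Arrived event sets the cube material to Mat_Screen.
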(event Custom|Arrived
  (Rendering|Material|SetMaterial (Variables|Default|GetCube) 0 "/Game/Blueprint/GPE/Quêtes/Sincronisation/Mat_Screen.Mat_Screen"))

(event EventBeginPlay
  (|CallParentFunction)
  (Rendering|Components|TextRender|SetText (Variables|Default|GetTextRender) (Utilities|Text|ToText(Integer) (Variables|Default|GetNumber)))
  (bind _returnvalue (Actor|GetActorOfClass "/Game/Blueprint/GPE/DecorationGPE/Assenseur/BP_Assenseur.BP_Assenseur_C"))
  (Variables|Default|SetAssenseur _returnvalue))

(event Collision|EventActorBeginOverlap
  (params (OtherActor :type Actor%20Object%20Reference))
  (|CallParentFunction OtherActor) ; This node is disabled and will not be called.\nDrag off pins to build functionality.
)

(event EventTick
  (params (DeltaSeconds :type Float%20%28single-precision%29))
  (|CallParentFunction DeltaSeconds) ; This node is disabled and will not be called.\nDrag off pins to build functionality.
)

(event EventInterract
  (params (First%20person%20ref :type BP%20First%20Person%20Character%20Object%20Reference))
  (bind _assenseur (Variables|Default|GetAssenseur))
  (if (!= (Variables|Default|GetNumber) (Variables|/Game/Blueprint/GPE/DecorationGPE/Assenseur/BP_Assenseur.BP_Assenseur_C|GetStage _assenseur))
    (if (not (Variables|/Game/Blueprint/GPE/DecorationGPE/Assenseur/BP_Assenseur.BP_Assenseur_C|GetMooving _assenseur))
      (Default|GotoStage (Variables|Default|GetAssenseur) (Variables|Default|GetNumber))
      (Rendering|Material|SetMaterial (Variables|Default|GetCube) 0 "/Game/Blueprint/GPE/Quêtes/Sincronisation/Mat_On.Mat_On"))))

(fn ConstructionScript
  (|CallParentFunction))