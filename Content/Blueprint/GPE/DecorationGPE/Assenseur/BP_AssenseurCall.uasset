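; BP_AssenseurCall is an elevator call button tied to one floor, which summons the referenced elevator when interacted with.
; Interract sends the elevator to SelfStage if it is on another stage and the Delay flag is set, then clears the flag and switches the Cube to its on material.
; Assensseurarrive re-arms the flag and restores the screen material, so repeat calls are ignored until that event fires.
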(event Custom|Assensseur%20arrive
  (Variables|Default|SetDelay true)
  (Rendering|Material|SetMaterial (Variables|Default|GetCube) 0 "/Game/Blueprint/GPE/Quêtes/Sincronisation/Mat_Screen.Mat_Screen"))

(event EventBeginPlay
  (|CallParentFunction) ; This node is disabled and will not be called.\nDrag off pins to build functionality.
)

(event Collision|EventActorBeginOverlap
  (params (OtherActor :type Actor%20Object%20Reference))
  (|CallParentFunction OtherActor) ; This node is disabled and will not be called.\nDrag off pins to build functionality.
)

(event EventTick
  (params (DeltaSeconds :type Float%20%28single-precision%29))
  (|CallParentFunction DeltaSeconds) ; This node is disabled and will not be called.\nDrag off pins to build functionality.
)

(event EventInterract
  (params (First%20person%20ref :type BP%20First%20Person%20Character%20Object%20Reference))
  (if (!= (Variables|/Game/Blueprint/GPE/DecorationGPE/Assenseur/BP_Assenseur.BP_Assenseur_C|GetStage (Variables|Default|GetAssenseur%20ref)) (Variables|Default|GetSelf%20stage))
    (if (Variables|Default|GetDelay)
      (Variables|Default|SetDelay false)
      (Default|GotoStage (Variables|Default|GetAssenseur%20ref) (Variables|Default|GetSelf%20stage))
      (Rendering|Material|SetMaterial (Variables|Default|GetCube) 0 "/Game/Blueprint/GPE/Quêtes/Sincronisation/Mat_On.Mat_On"))))

(fn ConstructionScript
  (|CallParentFunction))