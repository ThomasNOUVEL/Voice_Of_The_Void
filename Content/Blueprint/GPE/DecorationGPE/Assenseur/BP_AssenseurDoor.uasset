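; Elevator door actor for one floor, pairing two sliding panels with a child-actor call station.
; On BeginPlay it passes the elevator reference, its floor and itself to the BP_AssenseurCall child.
; Open and close events play a timeline forward or in reverse, lerping both panels' relative locations apart or together.
; When the timeline finishes in either direction, it records the open state and notifies the call station through AssensseurArrive.
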(event Custom|Close%20the%20Door
  (bind (_direction _float) (Timeline|Timeline ReverseFromEnd)
    (:Update
      (Transformation|SetRelativeLocation (Variables|Default|GetLeft%20Door) (Math|Vector|Lerp(Vector) "122.000000,30.000000,115.000000" "122.000000,82.000000,115.000000" _float) false false)
      (Transformation|SetRelativeLocation (Variables|Default|GetRight%20Door) (Math|Vector|Lerp(Vector) "122.000000,-30.000000,115.000000" "122.000000,-82.000000,115.000000" _float) false false))
    (:Finished
      (Variables|Default|SetOppen%20Close (Utilities|Select :Index _direction :Forward true :Backward false))
      (Default|AssensseurArrive (Variables|Default|GetAs%20BP%20Assenseur%20Call)))))

(event Custom|Oppen%20the%20door
  (bind (_direction _float) (Timeline|Timeline PlayFromStart)
    (:Update
      (Transformation|SetRelativeLocation (Variables|Default|GetLeft%20Door) (Math|Vector|Lerp(Vector) "122.000000,30.000000,115.000000" "122.000000,82.000000,115.000000" _float) false false)
      (Transformation|SetRelativeLocation (Variables|Default|GetRight%20Door) (Math|Vector|Lerp(Vector) "122.000000,-30.000000,115.000000" "122.000000,-82.000000,115.000000" _float) false false))
    (:Finished
      (Variables|Default|SetOppen%20Close (Utilities|Select :Index _direction :Forward true :Backward false))
      (Default|AssensseurArrive (Variables|Default|GetAs%20BP%20Assenseur%20Call)))))

(event EventBeginPlay
  (Variables|Default|SetAs%20BP%20Assenseur%20Call (.AsBP%20Assenseur%20Call (Utilities|Casting|CastToBP_AssenseurCall (Variables|/Script/Engine.ChildActorComponent|GetChildActor (Variables|Default|GetBP_AssenseurCall)))))
  (Variables|/Game/Blueprint/GPE/DecorationGPE/Assenseur/BP_AssenseurCall.BP_AssenseurCall_C|SetAssenseur%20ref (Variables|Default|GetAs%20BP%20Assenseur%20Call) (Variables|Default|GetAssensseur%20ref))
  (Variables|/Game/Blueprint/GPE/DecorationGPE/Assenseur/BP_AssenseurCall.BP_AssenseurCall_C|SetSelf%20stage (Variables|Default|GetAs%20BP%20Assenseur%20Call) (Variables|Default|GetEtage))
  (Variables|/Game/Blueprint/GPE/DecorationGPE/Assenseur/BP_AssenseurCall.BP_AssenseurCall_C|SetAssenseur%20door%20ref (Variables|Default|GetAs%20BP%20Assenseur%20Call) self))

(fn ConstructionScript)