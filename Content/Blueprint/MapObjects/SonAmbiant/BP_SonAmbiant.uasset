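; BP_SonAmbiant is a map object that plays an ambient sound in the level.
; On BeginPlay it stops its SonAmbian audio component, assigns SoundRef as the sound and calls LoopSound.
; LoopSound plays the component from the start once; the Delay-based replay using the sound's duration is disconnected, so the Blueprint itself does not repeat the sound.
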(event Custom|Loop%20Sound
  (Audio|Components|Audio|Play (Variables|Default|GetSonAmbian) 0.0))

(event EventBeginPlay
  (bind _sonambian (Variables|Default|GetSonAmbian))
  (Audio|Components|Audio|Stop _sonambian)
  (Audio|Components|Audio|SetSound _sonambian (Variables|Default|GetSound%20ref))
  (CallFunction|LoopSound))

(fn ConstructionScript)